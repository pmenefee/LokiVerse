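; ComplexController_Save handles persistence of a voxel world and its spawners through Save and Load functions.
; Save stores the world's compressed save and spawner save in the VoxelWorldSave and SpawnerSave variables.
; Load is currently empty: the nodes that restore the world, then its spawners, or print a failure message are disconnected and never run.
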(fn `Load`
  (params (`Voxel World` :type "VoxelWorld Object Reference")))

(fn `Save`
  (params (`Voxel World` :type "VoxelWorld Object Reference"))
  (bind _outsave (`VoxelDataTools.GetCompressedSave` `Voxel World`))
  (set `self.VoxelWorldSave` _outsave)
  (bind _returnvalue (`VoxelBlueprintLibrary.GetSpawnersSave` `Voxel World`))
  (set `self.SpawnerSave` _returnvalue))